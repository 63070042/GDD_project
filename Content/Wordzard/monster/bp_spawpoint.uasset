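; Monster spawn point that keeps a set number of BP_enemy characters populated inside its box area.
; On BeginPlay it disables box collision, spawns the initial batch and starts a looping timer that adds one enemy whenever ActivePawn is below SpwanAmount.
; SpawnCharacter line-traces downward from high above random box points to place each enemy on WorldStatic geometry, then assigns AIC_enemy, links it to this spawner and records it.
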(event `self.ReceiveBeginPlay`
  (`PrimitiveComponent.SetCollisionEnabled` (`self.Box`) "NoCollision")
  (for _ (range 1 (+ (`self.spwanAmount`) 1))
    (`self.Spawn Character`))
  (`KismetSystemLibrary.K2_SetTimer` null "RespawnCharacter" (`self.TimeTillRespawn`) true))

(fn `RespawnCharacter`
  (if (< (`KismetArrayLibrary.Array_Length` (`self.ActivePawn`)) (`self.spwanAmount`))
    (`self.Spawn Character`)))

(fn `Spawn Character`
  (bind (_origin _boxextent) (`KismetSystemLibrary.GetComponentBounds` (`self.Box`)))
  (bind _returnvalue (`KismetMathLibrary.MakeVector` (.x (`KismetMathLibrary.RandomPointInBoundingBox` _origin _boxextent)) (.y (`KismetMathLibrary.RandomPointInBoundingBox` _origin _boxextent)) (+ (.z (`KismetMathLibrary.RandomPointInBoundingBox` _origin _boxextent)) 10000.0)))
  (bind _outhit (`KismetSystemLibrary.LineTraceSingleForObjects` :`Start` _returnvalue :`End` (+ _returnvalue (* (* (`self.GetActorUpVector`) -1) 15000.0)) :`ObjectTypes` (`|MakeArray` "ObjectTypeQuery1" :!type "EObjectTypeQuery Enum") :`DrawDebugType` "ForDuration"))
  (bind _returnvalue_2 (`|SpawnActorFromClass` "/Game/TopDownBP/Blueprints/BP_enemy.BP_enemy_C" (`KismetMathLibrary.MakeTransform` (`.Location` (`GameplayStatics.BreakHitResult` _outhit)) (`KismetMathLibrary.MakeRotator` 0.0 0.0 (`KismetMathLibrary.RandomFloat`))) "AdjustIfPossibleButAlwaysSpawn" "OverrideRootScale" null null))
  (set `Pawn.AIControllerClass` "/Game/Wordzard/monster/AIC_enemy.AIC_enemy_C" _returnvalue_2)
  (`Pawn.SpawnDefaultController` _returnvalue_2)
  (set `/Game/TopDownBP/Blueprints/BP_enemy.SpawnPoint` self _returnvalue_2)
  (`KismetArrayLibrary.Array_Add` (`self.ActivePawn`) _returnvalue_2))

(fn `UserConstructionScript`)