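; Magic circle effect Blueprint with health and pawn sensing, whose Fx component takes its color parameter from the Color variable at construction.
; Damage subtracts from Health, and Tick destroys the actor only when Health equals exactly zero.
; Seeing an Urchest_BP runs AIMoveTo on that seen pawn, not this actor, with the same pawn as target actor and player 0's location as destination.
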(event `self.ReceiveTick`
  (params (DeltaSeconds :type "Float (single-precision)"))
  (`parent.ReceiveTick` DeltaSeconds)
  (if (== (`self.health`) 0.0)
    (`self.K2_DestroyActor`)))

(event `self.ReceiveAnyDamage`
  (params (Damage :type "Float (single-precision)") (DamageType :type "DamageType Object Reference") (InstigatedBy :type "Controller Object Reference") (DamageCauser :type "Actor Object Reference"))
  (set `self.health` (- (`self.health`) Damage)))

(event `self.PawnSensing.OnSeePawn`
  (params (Pawn :type "Pawn Object Reference"))
  (bind _asurchest_bp (cast `/Game/TopDownBP/Blueprints/Urchest_BP` Pawn))
  (`|AIMoveTo` Pawn (`self.K2_GetActorLocation` (`GameplayStatics.GetPlayerCharacter` 0)) _asurchest_bp 0.0))

(fn `UserConstructionScript`
  (`parent.UserConstructionScript`)
  (`ParticleSystemComponent.SetVectorParameter` (`self.fx`) "color" (`KismetMathLibrary.Conv_LinearColorToVector` (`self.color`))))