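; BP_ky_lightning2 is a lightning effect actor from FXVarietyPack that damages actors overlapping it.
; On ActorBeginOverlap it calls the parent handler, then applies damage to the other actor, randomized in a narrow range around its Damage variable.
; BeginPlay and Tick are disabled stubs, and the construction script only calls its parent.
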(event `self.ReceiveActorBeginOverlap`
  (params (OtherActor :type "Actor Object Reference"))
  (bind _damage (`self.Damage`))
  (`parent.ReceiveActorBeginOverlap` OtherActor)
  (`GameplayStatics.ApplyDamage` OtherActor (`KismetMathLibrary.RandomFloatInRange` (- _damage 3.0) (+ _damage 2.0))))

(fn `UserConstructionScript`
  (`parent.UserConstructionScript`))